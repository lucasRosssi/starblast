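; Gameplay ability that puts the hero into aiming for as long as the input is held.
; Activation applies GE_Aim to the owner and waits for input release, which ends the ability.
; On the locally controlled instance it caches the CameraDirector from CBP_Hero and switches its camera mode.
; Ending the ability removes the effect by its stored handle and sets the cached director to another camera mode.
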(event `self.K2_ActivateAbility`
  (bind _returnvalue (`self.BP_ApplyGameplayEffectToOwner` "/Game/Blueprints/AbilitySystem/GameplayEffects/CombatState/GE_Aim.GE_Aim_C"))
  (set `self.AimGEHandle` _returnvalue)
  (`AbilityTask_WaitInputRelease.WaitInputRelease` false
    (:`then`
      (`self.IsLocallyControlled`
        (:`True`
          (`/Engine/EditorBlueprintResources/StandardMacros.IsValid` (`self.Camera Director`)
            (:`Is Valid`
              (set `/Game/Blueprints/Cameras/CameraDirector_SandboxCharacter.CameraMode` "NewEnumerator2" (`self.Camera Director`) :!label _label))
            (:`Is Not Valid`
              (bind _ascbp_hero (cast `/Game/Blueprints/Characters/CBP_Hero` (`self.GetAvatarActorFromActorInfo`))
                (:`then`
                  (set `self.Camera Director` (`/Game/Blueprints/Characters/CBP_Hero.CameraDirector` _ascbp_hero))
                  (goto _label))
                (:`CastFailed`
                  (`self.K2_EndAbility`))))))))
    (:`OnRelease`
      (`self.K2_EndAbility`))))

(event `self.K2_OnEndAbility`
  (params (bWasCancelled :type Boolean))
  (`self.BP_RemoveGameplayEffectFromOwnerWithHandle` (`self.AimGEHandle`))
  (`/Engine/EditorBlueprintResources/StandardMacros.IsValid` (`self.Camera Director`)
    (:`Is Valid`
      (set `/Game/Blueprints/Cameras/CameraDirector_SandboxCharacter.CameraMode` "NewEnumerator1" (`self.Camera Director`)))))